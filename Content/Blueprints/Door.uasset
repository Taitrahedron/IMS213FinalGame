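; Folding garage door actor that starts locked and, once unlocked, raises when the third-person character enters its overlap and lowers when they leave.
; Two timelines offset the door's world Z from its starting position, while state flags block retriggering mid-move, so an exit during movement is ignored.
; An unlock event clears the lock, then turns the red status light green after a short delay.
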(event Custom|eventUnlockDoor
  (Variables|Default|SetdoorIsLocked false)
  (Utilities|FlowControl|Delay 0.75)
  (Rendering|Material|SetMaterial (Variables|Default|GetstatusLight) 0 "/Game/Materials/Green.Green"))

(event Custom|eventLowerDoor
  (Variables|Default|SetdoorIsUp false)
  (bind _garagedoorheight (Timeline|Lower%20the%20door PlayFromStart)
    (:Update
      (Transformation|SetWorldLocation (Variables|Default|GetfoldingDoor) (Math|Vector|MakeVector (Variables|Default|GetStartX) (Variables|Default|GetStartY) (+ _garagedoorheight (Variables|Default|GetStartZ))) false false))
    (:Finished
      (Variables|Default|SetdoorIsDown true)
      (Variables|Default|SetdoorIsMoving false))))

(event Custom|eventRaiseDoor
  (Variables|Default|SetdoorIsDown false)
  (bind _garagedoorheight (Timeline|Raise%20the%20door PlayFromStart)
    (:Update
      (Transformation|SetWorldLocation (Variables|Default|GetfoldingDoor) (Math|Vector|MakeVector (Variables|Default|GetStartX) (Variables|Default|GetStartY) (+ _garagedoorheight (Variables|Default|GetStartZ))) false false))
    (:Finished
      (Variables|Default|SetdoorIsUp true)
      (Variables|Default|SetdoorIsMoving false))))

(event EventBeginPlay
  (bind _foldingdoor (Variables|Default|GetfoldingDoor))
  (bind _returnvalue (Transformation|GetWorldLocation _foldingdoor))
  (Variables|Default|SetStartX (.x _returnvalue))
  (Variables|Default|SetStartY (.y _returnvalue))
  (Variables|Default|SetStartZ (.z _returnvalue))
  (Variables|Default|SetdoorIsDown true)
  (Variables|Default|SetdoorIsUp false)
  (Variables|Default|SetdoorIsMoving false)
  (Variables|Default|SetdoorIsLocked true)
  (Rendering|Material|SetMaterialbyName (Variables|Default|GetstatusLight) "None" "/Game/Materials/Red.Red"))

(event Collision|EventActorBeginOverlap
  (params (OtherActor :type Actor%20Object%20Reference))
  (Utilities|Casting|CastToBP_ThirdPersonCharacter OtherActor)
  (if (not (Variables|Default|GetdoorIsLocked))
    (if (not (Variables|Default|GetdoorIsMoving))
      (if (not (Variables|Default|GetdoorIsUp))
        (if (Variables|Default|GetdoorIsDown)
          (Variables|Default|SetdoorIsMoving true)
          (CallFunction|EventRaiseDoor)
          (Audio|PlaySound2D "/Game/Audio/doors.doors" 1.0 1.0 0.0 0 0))))))

(event Collision|EventActorEndOverlap
  (params (OtherActor :type Actor%20Object%20Reference))
  (Utilities|Casting|CastToBP_ThirdPersonCharacter OtherActor)
  (if (not (Variables|Default|GetdoorIsLocked))
    (if (not (Variables|Default|GetdoorIsMoving))
      (if (Variables|Default|GetdoorIsUp)
        (Variables|Default|SetdoorIsMoving true)
        (CallFunction|EventLowerDoor)
        (Audio|PlaySound2D "/Game/Audio/doors.doors" 1.0 1.0 0.0 0 0)))))

(fn ConstructionScript)