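; Actor Blueprint that moves itself, apparently a kart, along a path spline once play begins.
; BeginPlay caches the spline length from KartPathRef, then plays a timeline whose alpha maps to distance along the spline.
; Each update sets the actor transform to that world location, without following spline rotation.
; The GetActorOfClass lookup that would assign KartPathRef is disconnected and never runs.
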(event Custom|PlayKartTimeline
  (bind _kartmovement (Timeline|KartTimeline Play)
    (:Update
      (Transformation|SetActorTransform (Math|Transform|MakeTransform (Spline|GetLocationatDistanceAlongSpline (Variables|/Game/Blueprints/MovementPath.MovementPath_C|GetSpline (Variables|Default|GetKartPathRef)) (Math|Float|Lerp 0.0 (Variables|Default|GetKartPathLength) _kartmovement) "World") "0, 0, 0" "1.000000,1.000000,1.000000")))))

(event EventBeginPlay
  (Variables|Default|SetKartPathLength (Spline|GetSplineLength (Variables|/Game/Blueprints/MovementPath.MovementPath_C|GetSpline (Variables|Default|GetKartPathRef))))
  (CallFunction|PlayKartTimeline))

(fn ConstructionScript)